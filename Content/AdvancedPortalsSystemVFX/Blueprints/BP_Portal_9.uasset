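; Portal VFX actor that plays a material dissolve on its static mesh at BeginPlay, then switches on its effects.
; Dynamic material instances on two mesh slots, both sourced from slot 0, have their Dissolve parameter driven by a timeline.
; When the timeline finishes, the vortex and three spark components activate.
; The construction script applies one Scale value to the actor and the mesh's child Niagara systems.
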(event EventBeginPlay
  (Utilities|FlowControl|Sequence
    (:then_0
      (Rendering|Material|SetMaterial (Variables|Default|GetStaticMesh) 0 "/Game/Assets/Materials/MT_Dissolve_Inst.MT_Dissolve_Inst")
      (bind _returnvalue (Rendering|Material|CreateDynamicMaterialInstance (Variables|Default|GetStaticMesh) 0 (Rendering|Material|GetMaterial (Variables|Default|GetStaticMesh) 0) "None" :!class /Script/Engine.PrimitiveComponent))
      (Variables|Default|SetMaterial _returnvalue))
    (:then_1
      (bind _returnvalue_2 (Rendering|Material|CreateDynamicMaterialInstance (Variables|Default|GetStaticMesh) 1 (Rendering|Material|GetMaterial (Variables|Default|GetStaticMesh) 0) "None" :!class /Script/Engine.PrimitiveComponent))
      (Variables|Default|SetMaterial2 _returnvalue_2)
      (bind _time (Timeline|타임라인 PlayFromStart)
        (:Update
          (Rendering|Material|SetScalarParameterValue (Variables|Default|GetMaterial) "Dissolve" (Math|Float|Lerp 0.0 2.0 _time) :!class /Script/Engine.MaterialInstanceDynamic)
          (Rendering|Material|SetScalarParameterValue (Variables|Default|GetMaterial2) "Dissolve" (Math|Float|Lerp 0.0 2.0 _time) :!class /Script/Engine.MaterialInstanceDynamic))
        (:Finished
          (Components|Activation|SetActive (Variables|Default|GetVortex) true false)
          (Components|Activation|SetActive (Variables|Default|GetSparks_1) true false)
          (Components|Activation|SetActive (Variables|Default|GetSparks_2) true false)
          (Components|Activation|SetActive (Variables|Default|GetSparks_3) true false))))))

(fn ConstructionScript
  (for _array_element (Components|GetChildrenComponents (Variables|Default|GetStaticMesh) true)
    (bind _as나이아가라_파티클_시스템_컴포넌트 (Utilities|Casting|CastToNiagaraComponent _array_element))
    (Effects|Components|ParticleSystem|SetFloatParameter _as나이아가라_파티클_시스템_컴포넌트 "--Scale" (Variables|Default|GetScale)))
  (Transformation|SetActorScale3D (Math|Conversions|ToVector(Float) (Variables|Default|GetScale))))