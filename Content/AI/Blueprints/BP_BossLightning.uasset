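; BP_BossLightning is a boss lightning hazard actor that rotates a little every tick and expires after a fixed lifespan.
; When its capsule overlaps the tagged player character, it starts a joyful jump montage on the player's mesh and calls the character's Collision function.
; Vector-based and timeline-driven movement logic remains in the graph but is never run.
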(event OnBeginCursorOver(StaticMesh)
  (params (TouchedComponent :type Primitive%20Component%20Object%20Reference)))

(event OnComponentBeginOverlap(Capsule)
  (params (OverlappedComponent :type Primitive%20Component%20Object%20Reference) (OtherActor :type Actor%20Object%20Reference) (OtherComp :type Primitive%20Component%20Object%20Reference) (OtherBodyIndex :type Integer) (bFromSweep :type Boolean) (SweepResult :type Hit%20Result%20Structure%20%28by%20ref%29))
  (if (Actor|ActorHasTag OtherActor "Player")
    (bind _asbp_third_person_character (Utilities|Casting|CastToBP_ThirdPersonCharacter OtherActor))
    (Animation|Montage|PlayMontage (Variables|/Script/Engine.Character|GetMesh (Game|GetPlayerCharacter 0)) "/Game/Blueprints/Anime/VRM_M_Joyful_Jump_Montage.VRM_M_Joyful_Jump_Montage"
      (:then
        (Default|Collision _asbp_third_person_character)))))

(event EventBeginPlay
  (Actor|SetLifeSpan 2e+01))

(event Collision|EventActorBeginOverlap
  (params (OtherActor :type Actor%20Object%20Reference)))

(event EventTick
  (params (DeltaSeconds :type Float%20%28single-precision%29))
  (Class|Actor|AddActorWorldRotation "0.000000,1.000000,0.000000"))

(fn ConstructionScript)