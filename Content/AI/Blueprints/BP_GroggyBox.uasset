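; BP_GroggyBox is a short-lived trigger box in the boss fight that fires a star toward the boss when the player touches it.
; On Box1 overlap with BP_ThirdPersonCharacter, it calls LaunchBoss on that character, spawns a BP_Star and destroys itself.
; The star's velocity comes from SuggestProjectileVelocity, aimed at a point above the BP_BossCharacter found in the level.
; An untouched box expires through a lifespan set on BeginPlay.
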(event OnComponentBeginOverlap(Box1)
  (params (OverlappedComponent :type Primitive%20Component%20Object%20Reference) (OtherActor :type Actor%20Object%20Reference) (OtherComp :type Primitive%20Component%20Object%20Reference) (OtherBodyIndex :type Integer) (bFromSweep :type Boolean) (SweepResult :type Hit%20Result%20Structure%20%28by%20ref%29))
  (bind _asbp_third_person_character (Utilities|Casting|CastToBP_ThirdPersonCharacter OtherActor))
  (Default|LaunchBoss _asbp_third_person_character)
  (bind _returnvalue (Actor|GetActorOfClass "/Game/MPMECH/BP/BP_BossCharacter.BP_BossCharacter_C"))
  (bind _tossvelocity (Class|GameplayStatics|BlueprintSuggestProjectileVelocity (Transformation|GetActorLocation) (Math|Vector|MakeVector (.x (Transformation|GetActorLocation _returnvalue)) (.y (Transformation|GetActorLocation _returnvalue)) (+ (.z (Transformation|GetActorLocation _returnvalue)) 5e+02)) 1.2e+03 0.5 "DoNotTrace" 0.0 false false false))
  (Game|SpawnActorfromClass "/Game/AI/Blueprints/BP_Star.BP_Star_C" (Transformation|GetActorTransform) "Undefined" "MultiplyWithRoot" 0 _tossvelocity 0)
  (Actor|DestroyActor))

(event EventBeginPlay
  (Actor|SetLifeSpan 1e+01))

(event Collision|EventActorBeginOverlap
  (params (OtherActor :type Actor%20Object%20Reference)))

(event EventTick
  (params (DeltaSeconds :type Float%20%28single-precision%29)))

(fn ConstructionScript)