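; BP_RayzerBeam is a short-lived laser beam hazard that arms itself after a delay and affects the third-person character.
; Tick accumulates time until it exceeds Cooldown, then a one-shot flag activates the Beam component, plays SuperLaser and enables overlap events on the capsule.
; Capsule overlaps with BP_ThirdPersonCharacter call that character's Collision function.
; A lifespan set on BeginPlay destroys the actor automatically.
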(event OnComponentBeginOverlap(Capsule)
  (params (OverlappedComponent :type Primitive%20Component%20Object%20Reference) (OtherActor :type Actor%20Object%20Reference) (OtherComp :type Primitive%20Component%20Object%20Reference) (OtherBodyIndex :type Integer) (bFromSweep :type Boolean) (SweepResult :type Hit%20Result%20Structure%20%28by%20ref%29))
  (bind _asbp_third_person_character (Utilities|Casting|CastToBP_ThirdPersonCharacter OtherActor))
  (Default|Collision _asbp_third_person_character))

(event EventBeginPlay
  (Actor|SetLifeSpan 7.0))

(event Collision|EventActorBeginOverlap
  (params (OtherActor :type Actor%20Object%20Reference)))

(event EventTick
  (params (DeltaSeconds :type Float%20%28single-precision%29))
  (if (not (Variables|Default|GetNewVar))
    (bind _output_get (Variables|Default|SetCurrentTime (+ DeltaSeconds (Variables|Default|GetCurrentTime))))
    (if (> _output_get (Variables|Default|Getcooldown))
      (Components|Activation|SetActive (Variables|Default|GetBeam) true false)
      (Audio|Components|Audio|Play (Variables|Default|GetsuperLaser) 0.0)
      (Variables|/Script/Engine.PrimitiveComponent|SetbGenerateOverlapEvents (Variables|Default|GetCapsule) true)
      (Variables|Default|SetNewVar true))))

(fn ConstructionScript)