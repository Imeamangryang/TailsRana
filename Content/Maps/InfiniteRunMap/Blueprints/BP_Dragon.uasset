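; Dragon actor for the infinite run map that flies along +X and shows the infinite-mode goal UI when the player reaches it.
; On BeginPlay it moves 2000 units ahead of the player in X, matching their Y, then starts its StateTree after five seconds.
; Tick advances it by Speed, scaled by delta time.
; A Box overlap with the third-person character triggers the goal display through the player HUD.
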(event OnComponentBeginOverlap(Box)
  (params (OverlappedComponent :type Primitive%20Component%20Object%20Reference) (OtherActor :type Actor%20Object%20Reference) (OtherComp :type Primitive%20Component%20Object%20Reference) (OtherBodyIndex :type Integer) (bFromSweep :type Boolean) (SweepResult :type Hit%20Result%20Structure%20%28by%20ref%29))
  (Utilities|Casting|CastToBP_ThirdPersonCharacter OtherActor)
  (bind _ashud_uitest_player_hud (Utilities|Casting|CastToHUD_UITestPlayerHUD (HUD|GetHUD (Game|GetPlayerController 0))))
  (Default|VisibleGoalUIInfinite _ashud_uitest_player_hud))

(event EventBeginPlay
  (bind _returnvalue (Game|GetPlayerCharacter 0))
  (bind _returnvalue_2 (Transformation|GetActorLocation _returnvalue))
  (Transformation|SetActorLocation (Math|Vector|MakeVector (+ (.x _returnvalue_2) 2e+03) (.y _returnvalue_2) 0.0) false false)
  (Utilities|FlowControl|Delay 5.0)
  (AI|Logic|StartLogic (Variables|Default|GetStateTree)))

(event EventTick
  (params (DeltaSeconds :type Float%20%28single-precision%29))
  (bind _returnvalue (Transformation|GetActorLocation))
  (Transformation|SetActorLocation (Math|Vector|MakeVector (+ (.x _returnvalue) (* DeltaSeconds (Variables|Default|GetSpeed))) (.y _returnvalue) (.z _returnvalue)) false false))

(fn ConstructionScript)