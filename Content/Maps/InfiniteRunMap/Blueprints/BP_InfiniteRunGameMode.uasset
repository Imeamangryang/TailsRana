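; Game mode for an infinite runner map that builds and recycles the floor track.
; On BeginPlay it spawns a start floor, pre-spawns a batch of tiles and caches the dragon actor.
; Each new tile is a weighted random pick between regular and escape floors, chained through the previous tile's attach point.
; ExtendFloor adds a tile and destroys the oldest once it is far enough from the dragon along X.
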(event EventBeginPlay
  (bind _returnvalue (Game|SpawnActorfromClass "/Game/Maps/InfiniteRunMap/Blueprints/BP_StartFloor.BP_StartFloor_C" (Variables|Default|GetFloor%20AttachPoint) "Undefined" "MultiplyWithRoot" 0 0))
  (bind _returnvalue_2 (Default|GetAttachPoint _returnvalue))
  (Variables|Default|SetFloor%20AttachPoint _returnvalue_2)
  (Utilities|Array|Add (Variables|Default|GetFloor%20Tiles) _returnvalue)
  (for _index (range 0 (- (Variables|Default|GetTileSpawnNumber) 1))
    (CallFunction|AddFloor)
    (bind _returnvalue_3 (Actor|GetActorOfClass "/Game/Maps/InfiniteRunMap/Blueprints/BP_OutDragon.BP_OutDragon_C"))
    (Variables|Default|SetDragon _returnvalue_3)))

(fn ConstructionScript)

(fn AddFloor
  (if (< (Math|Random|RandomFloatinRange 0.0 1.0) 0.8)
    (bind _returnvalue (Game|SpawnActorfromClass "/Game/Maps/InfiniteRunMap/Blueprints/BP_Floor.BP_Floor_C" (Variables|Default|GetFloor%20AttachPoint) "Undefined" "MultiplyWithRoot" 0 0))
    (bind _returnvalue_2 (Default|GetAttachPoint _returnvalue))
    (Variables|Default|SetFloor%20AttachPoint _returnvalue_2)
    (Utilities|Array|Add (Variables|Default|GetFloor%20Tiles) _returnvalue)
    (else
      (bind _returnvalue_3 (Game|SpawnActorfromClass "/Game/Maps/InfiniteRunMap/Blueprints/BP_EscapeFloor.BP_EscapeFloor_C" (Variables|Default|GetFloor%20AttachPoint) "Undefined" "MultiplyWithRoot" 0 0))
      (bind _returnvalue_4 (Default|GetAttachPoint _returnvalue_3))
      (Variables|Default|SetFloor%20AttachPoint _returnvalue_4)
      (Utilities|Array|Add (Variables|Default|GetFloor%20Tiles) _returnvalue_3))))

(fn ExtendFloor
  (bind _floor_tiles (Variables|Default|GetFloor%20Tiles))
  (bind _output (Utilities|Array|Get(acopy) _floor_tiles))
  ;[0.15 0.15 0.15 0.5] 일정 수 이하일  때 생성
  (CallFunction|AddFloor)
  (if (> (Math|Float|Absolute(Float) (- (.x (Transformation|GetActorLocation (Utilities|Array|Get(acopy) (Variables|Default|GetFloor%20Tiles)))) (.x (Transformation|GetActorLocation (Variables|Default|GetDragon))))) 5e+03)
    (Actor|DestroyActor _output)
    (Utilities|Array|RemoveItem _floor_tiles _output)))