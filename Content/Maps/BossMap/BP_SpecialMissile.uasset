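; BP_SpecialMissile is a boss-map projectile that falls straight down at a constant speed, moved every Tick without sweep.
; When its capsule overlaps the player character tagged "Player", it calls VisibleOutUIBoss on the player HUD.
; When it overlaps an actor tagged "Fixed", it destroys both that actor and itself.
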(event OnComponentBeginOverlap(Capsule)
  (params (OverlappedComponent :type Primitive%20Component%20Object%20Reference) (OtherActor :type Actor%20Object%20Reference) (OtherComp :type Primitive%20Component%20Object%20Reference) (OtherBodyIndex :type Integer) (bFromSweep :type Boolean) (SweepResult :type Hit%20Result%20Structure%20%28by%20ref%29))
  (Utilities|FlowControl|Sequence
    (:then_0
      (if (Actor|ActorHasTag OtherActor "Player")
        (Utilities|Casting|CastToBP_ThirdPersonCharacter OtherActor)
        (bind _ashud_uitest_player_hud (Utilities|Casting|CastToHUD_UITestPlayerHUD (HUD|GetHUD (Game|GetPlayerController 0))))
        (Default|VisibleOutUIBoss _ashud_uitest_player_hud)))
    (:then_1
      (if (Actor|ActorHasTag OtherActor "Fixed")
        (Actor|DestroyActor OtherActor)
        (Actor|DestroyActor)))))

(event EventBeginPlay)

(event Collision|EventActorBeginOverlap
  (params (OtherActor :type Actor%20Object%20Reference)))

(event EventTick
  (params (DeltaSeconds :type Float%20%28single-precision%29))
  (Transformation|SetActorLocation (+ (Transformation|GetActorLocation) (* DeltaSeconds 1.5e+03 (Math|Vector|MakeVector 0.0 0.0 -1.0))) false false))

(fn ConstructionScript)