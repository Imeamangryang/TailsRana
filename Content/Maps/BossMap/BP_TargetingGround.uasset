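; BP_TargetingGround is a boss-map ground targeting marker that follows the player and then calls down a missile.
; It snaps to the player's XY just above zero height on BeginPlay and on each Tick while IsTargeting is set, accumulating elapsed time.
; After five seconds it stops following and spawns BP_TargetingMissile high above the player's current position.
; The marker stays in place afterward, with no destroy logic here.
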(event EventBeginPlay
  (bind _returnvalue (Game|GetPlayerCharacter 0))
  (bind _returnvalue_2 (Transformation|GetActorLocation _returnvalue))
  (Transformation|SetActorLocation (Math|Vector|MakeVector (.x _returnvalue_2) (.y _returnvalue_2) 0.1) false false))

(event EventTick
  (params (DeltaSeconds :type Float%20%28single-precision%29))
  (bind _returnvalue (Game|GetPlayerCharacter 0))
  (bind _returnvalue_2 (Game|GetPlayerCharacter 0))
  (bind _returnvalue_3 (Transformation|GetActorLocation _returnvalue_2))
  (bind _returnvalue_4 (Transformation|GetActorLocation _returnvalue))
  (if (Variables|Default|GetIsTargeting)
    (bind _output_get (Variables|Default|SetLifeSpan (+ DeltaSeconds (Variables|Default|GetLifeSpan))))
    (if (< _output_get 5.0)
      (Transformation|SetActorLocation (Math|Vector|MakeVector (.x _returnvalue_4) (.y _returnvalue_4) 0.1) false false)
      (else
        (Variables|Default|SetIsTargeting false)
        (bind _output_get_2 (Variables|Default|SetTargetLocation (Math|Vector|MakeVector (.x _returnvalue_3) (.y _returnvalue_3) 5e+03)))
        (Game|SpawnActorfromClass "/Game/Maps/BossMap/BP_TargetingMissile.BP_TargetingMissile_C" (Math|Transform|MakeTransform _output_get_2 "0, 0, 0" "1.000000,1.000000,1.000000") "Undefined" "MultiplyWithRoot" 0 0)))))

(fn ConstructionScript)