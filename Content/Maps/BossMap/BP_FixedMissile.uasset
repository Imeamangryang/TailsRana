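; BP_FixedMissile is a boss-map projectile that falls straight down at constant speed, moved each Tick without sweep.
; Its capsule overlap calls Collision on the third-person character when it hits a Player-tagged actor, without destroying the missile.
; Overlapping a Fixed-tagged actor plays an explosion sound, spawns a Niagara hit effect below the missile, and destroys both that actor and the missile.
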(event OnComponentBeginOverlap(Capsule)
  (params (OverlappedComponent :type Primitive%20Component%20Object%20Reference) (OtherActor :type Actor%20Object%20Reference) (OtherComp :type Primitive%20Component%20Object%20Reference) (OtherBodyIndex :type Integer) (bFromSweep :type Boolean) (SweepResult :type Hit%20Result%20Structure%20%28by%20ref%29))
  (bind _returnvalue (Transformation|GetActorLocation))
  (Utilities|FlowControl|Sequence
    (:then_0
      (if (Actor|ActorHasTag OtherActor "Player")
        (bind _asbp_third_person_character (Utilities|Casting|CastToBP_ThirdPersonCharacter OtherActor))
        (Default|Collision _asbp_third_person_character)))
    (:then_1
      (if (Actor|ActorHasTag OtherActor "Fixed")
        (Audio|PlaySoundatLocation "/Game/Assets/Sounds/Boss/explosion.explosion" _returnvalue "0, 0, 0" 1.0 1.0 0.0 0 0 0 0)
        (Niagara|SpawnSystematLocation "/Game/sA_Megapack_v1/sA_StylizedAttacksPack/FX/NiagaraSystems/NS_BasicHit1.NS_BasicHit1" (- _returnvalue "0.000000,0.000000,700.000000"))
        (Actor|DestroyActor OtherActor)
        (Actor|DestroyActor)))))

(event EventBeginPlay)

(event Collision|EventActorBeginOverlap
  (params (OtherActor :type Actor%20Object%20Reference)))

(event EventTick
  (params (DeltaSeconds :type Float%20%28single-precision%29))
  (Transformation|SetActorLocation (+ (Transformation|GetActorLocation) (* DeltaSeconds 2e+03 (Math|Vector|MakeVector 0.0 0.0 -1.0))) false false))

(fn ConstructionScript)