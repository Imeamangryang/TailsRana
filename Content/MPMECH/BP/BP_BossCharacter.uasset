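; Boss character with health and groggy meters, beam anchor points, thruster and groggy effects, and a StateTree started through a function.
; Capsule hits cost health and groggy before the player cast, then launch the player with impact effects; a failed cast leaves IsHit set.
; Dispatchers broadcast meter changes, and zero health shows the boss goal UI and destroys the actor.
; Random-turn rotation logic is disconnected.
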(event OnComponentHit(CapsuleComponent)
  (params (HitComponent :type Primitive%20Component%20Object%20Reference) (OtherActor :type Actor%20Object%20Reference) (OtherComp :type Primitive%20Component%20Object%20Reference) (NormalImpulse :type Vector :default "0, 0, 0") (Hit :type Hit%20Result%20Structure%20%28by%20ref%29))
  ;[0.15 0.15 0.15 0.5] 캐릭터와 부딪혔을 때 충돌 처리
  (if (not (Variables|Default|GetIsHit))
    (Variables|Default|SetIsHit true)
    (CallFunction|BossApplyDamage)
    (CallFunction|BossApplyGroggyCoillsion)
    (bind _asbp_third_person_character (Utilities|Casting|CastToBP_ThirdPersonCharacter OtherActor))
    (Default|LaunchBoss _asbp_third_person_character)
    (Variables|Default|SetIsHit false)
    (Audio|PlaySoundatLocation "/Game/Assets/Sounds/Boss/aoeBlast.aoeBlast" (Transformation|GetActorLocation _asbp_third_person_character) "0, 0, 0" 1e+01 1.0 0.0 0 0 0 0)
    (Niagara|SpawnSystematLocation "/Game/sA_Megapack_v1/sA_StylizedAttacksPack/FX/NiagaraSystems/NS_BasicHit.NS_BasicHit" (+ (Transformation|GetActorLocation _asbp_third_person_character) "0.000000,0.000000,50.000000"))))

(event EventBeginPlay
  (CallFunction|SpawnEnergyBeamSign))

(event EventTick
  (params (DeltaSeconds :type Float%20%28single-precision%29)))

(fn ConstructionScript)

(fn BossApplyDamage
  (bind _result (Math|Float|DecrementFloat (Variables|Default|GetHealth))
    (:%20%20
      (Default|CallHealthDispatcher _result (Variables|Default|GetMaxHealth))
      (if (== (Variables|Default|GetHealth) 0)
        ;[0.15 0.15 0.15 0.5] GoalUI 불러오기
        (EventDispatchers|UnbindallEventsfromHealthDispatcher)
        (bind _ashud_uitest_player_hud (Utilities|Casting|CastToHUD_UITestPlayerHUD (HUD|GetHUD (Game|GetPlayerController 0))))
        (Default|VisibleGoalUIBoss _ashud_uitest_player_hud)
        (Actor|DestroyActor)))))

(fn NewRotation
  (bind _returnvalue (Transformation|GetActorLocation))
  (Variables|Default|SetTargetRotation (Math|Rotator|MakeRotator (.x _returnvalue) (.y _returnvalue) (+ (.z _returnvalue) (* (Math|Random|RandomFloatinRange 9e+01 3.6e+02) (.OutItem (Utilities|Array|Random (Variables|Default|GetTarget%20Yaw%20Offset))))))))

(fn StartStateTree
  (AI|Logic|StartLogic (Variables|Default|GetStateTree)))

(fn BossApplyGroggy
  (bind _result (Math|Float|DecrementFloat (Variables|Default|GetGroggy))
    (:%20%20
      (Default|CallGroggyDispatcher _result (Variables|Default|GetMaxGroggy)))))

(fn GroggyBoss
  (bind _output_get (Variables|Default|SetGroggy (Variables|Default|GetMaxGroggy)))
  (Default|CallGroggyDispatcher _output_get (Variables|Default|GetMaxGroggy)))

(fn SpawnEnergyBeamSign
  (Variables|Default|SetRayzerTransform (Utilities|Array|MakeArray (Transformation|GetWorldTransform (Variables|Default|GetScene)) (Transformation|GetWorldTransform (Variables|Default|GetScene1)) (Transformation|GetWorldTransform (Variables|Default|GetScene2)) (Transformation|GetWorldTransform (Variables|Default|GetScene3)) (Transformation|GetWorldTransform (Variables|Default|GetScene4)) (Transformation|GetWorldTransform (Variables|Default|GetScene5)))))

(fn ActiveThruster
  (Components|Activation|SetActive (Variables|Default|GetNiagara) true false)
  (Animation|PlayAnimMontage "/Game/MPMECH/BP/MM_Fall_Loop_ANIM_Montage.MM_Fall_Loop_ANIM_Montage" 1.0 "None"))

(fn DeactiveThruster
  (Components|Activation|SetActive (Variables|Default|GetNiagara) false false)
  (Animation|StopAnimMontage "/Game/MPMECH/BP/MM_Fall_Loop_ANIM_Montage.MM_Fall_Loop_ANIM_Montage"))

(fn BossApplyGroggyCoillsion
  (bind _output_get (Variables|Default|SetGroggy (- (Variables|Default|GetGroggy) 0.5)))
  (Default|CallGroggyDispatcher _output_get (Variables|Default|GetMaxGroggy)))

(fn ActiveGroggy
  (Components|Activation|SetActive (Variables|Default|GetGroggyEffect) true false))

(fn DeactiveGroggy
  (Components|Activation|SetActive (Variables|Default|GetGroggyEffect) false false))