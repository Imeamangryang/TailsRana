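; StateTree task that fires a sweeping fireball attack pattern, spawning BP_FireBall_1 actors relative to a referenced actor's transform.
; On entering the state, a timed chain of delays and spawns steps through five Y/Z offset slots, sweeping back and forth twice.
; The middle spawn, at the first slot, has no class set.
; The task finishes successfully after the last spawn.
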(event EventLatentEnterState
  (params (Transition :type State%20Tree%20Transition%20Result%20Structure%20%28by%20ref%29))
  (bind _123 (Variables|Context|Get123))
  (bind _123_2 (Variables|Context|Get123))
  (bind _123_3 (Variables|Context|Get123))
  (bind _123_4 (Variables|Context|Get123))
  (bind _123_5 (Variables|Context|Get123))
  (bind _123_6 (Variables|Context|Get123))
  (bind _123_7 (Variables|Context|Get123))
  (bind _123_8 (Variables|Context|Get123))
  (bind _123_9 (Variables|Context|Get123))
  (bind _123_10 (Variables|Context|Get123))
  (bind _123_11 (Variables|Context|Get123))
  (bind _123_12 (Variables|Context|Get123))
  (bind _123_13 (Variables|Context|Get123))
  (bind _123_14 (Variables|Context|Get123))
  (bind _123_15 (Variables|Context|Get123))
  (bind _123_16 (Variables|Context|Get123))
  (bind _123_17 (Variables|Context|Get123))
  (bind _returnvalue (Transformation|GetActorTransform _123_9))
  (bind _returnvalue_2 (Transformation|GetActorTransform _123_17))
  (bind _returnvalue_3 (Transformation|GetActorTransform _123_3))
  (bind _returnvalue_4 (Transformation|GetActorTransform _123_16))
  (bind _returnvalue_5 (Transformation|GetActorTransform _123_2))
  (bind _returnvalue_6 (Transformation|GetActorTransform _123_4))
  (bind _returnvalue_7 (Transformation|GetActorTransform _123_5))
  (bind _returnvalue_8 (Transformation|GetActorTransform _123))
  (bind _returnvalue_9 (Transformation|GetActorTransform _123_6))
  (bind _returnvalue_10 (Transformation|GetActorTransform _123_7))
  (bind _returnvalue_11 (Transformation|GetActorTransform _123_8))
  (bind _returnvalue_12 (Transformation|GetActorTransform _123_10))
  (bind _returnvalue_13 (Transformation|GetActorTransform _123_15))
  (bind _returnvalue_14 (Transformation|GetActorTransform _123_11))
  (bind _returnvalue_15 (Transformation|GetActorTransform _123_12))
  (bind _returnvalue_16 (Transformation|GetActorTransform _123_13))
  (bind _returnvalue_17 (Transformation|GetActorTransform _123_14))
  (Utilities|FlowControl|Delay 0.2)
  (Game|SpawnActorfromClass "/Game/Blueprints/Maps/BP_FireBall_1.BP_FireBall_1_C" (Math|Transform|MakeTransform (Math|Vector|MakeVector (.x (.location _returnvalue_7)) (- (.y (.location _returnvalue_7)) (Variables|Default|GetYVar1)) (+ (.z (.location _returnvalue_7)) (Variables|Default|GetZVar1))) (.rotation _returnvalue_7) (.scale _returnvalue_7)) "Undefined" "MultiplyWithRoot" 0 0)
  (Utilities|FlowControl|Delay 0.2)
  (Game|SpawnActorfromClass "/Game/Blueprints/Maps/BP_FireBall_1.BP_FireBall_1_C" (Math|Transform|MakeTransform (Math|Vector|MakeVector (.x (.location _returnvalue_9)) (- (.y (.location _returnvalue_9)) (Variables|Default|GetYVar2)) (+ (.z (.location _returnvalue_9)) (Variables|Default|GetZVar2))) (.rotation _returnvalue_9) (.scale _returnvalue_9)) "Undefined" "MultiplyWithRoot" 0 0)
  (Utilities|FlowControl|Delay 0.2)
  (Game|SpawnActorfromClass "/Game/Blueprints/Maps/BP_FireBall_1.BP_FireBall_1_C" (Math|Transform|MakeTransform (Math|Vector|MakeVector (.x (.location _returnvalue_10)) (- (.y (.location _returnvalue_10)) (Variables|Default|GetYVar3)) (+ (.z (.location _returnvalue_10)) (Variables|Default|GetZVar3))) (.rotation _returnvalue_10) (.scale _returnvalue_10)) "Undefined" "MultiplyWithRoot" 0 0)
  (Utilities|FlowControl|Delay 0.2)
  (Game|SpawnActorfromClass "/Game/Blueprints/Maps/BP_FireBall_1.BP_FireBall_1_C" (Math|Transform|MakeTransform (Math|Vector|MakeVector (.x (.location _returnvalue_11)) (+ (Variables|Default|GetYVar4) (.y (.location _returnvalue_11))) (+ (.z (.location _returnvalue_11)) (Variables|Default|GetZVar4))) (.rotation _returnvalue_11) (.scale _returnvalue_11)) "Undefined" "MultiplyWithRoot" 0 0)
  (Utilities|FlowControl|Delay 0.2)
  (Game|SpawnActorfromClass "/Game/Blueprints/Maps/BP_FireBall_1.BP_FireBall_1_C" (Math|Transform|MakeTransform (Math|Vector|MakeVector (.x (.location _returnvalue_12)) (+ (Variables|Default|GetYVar5) (.y (.location _returnvalue_12))) (+ (.z (.location _returnvalue_12)) (Variables|Default|GetZVar5))) (.rotation _returnvalue_12) (.scale _returnvalue_12)) "Undefined" "MultiplyWithRoot" 0 0)
  (Utilities|FlowControl|Delay 0.2)
  (Game|SpawnActorfromClass "/Game/Blueprints/Maps/BP_FireBall_1.BP_FireBall_1_C" (Math|Transform|MakeTransform (Math|Vector|MakeVector (.x (.location _returnvalue_14)) (+ (Variables|Default|GetYVar4) (.y (.location _returnvalue_14))) (+ (.z (.location _returnvalue_14)) (Variables|Default|GetZVar4))) (.rotation _returnvalue_14) (.scale _returnvalue_14)) "Undefined" "MultiplyWithRoot" 0 0)
  (Utilities|FlowControl|Delay 0.2)
  (Game|SpawnActorfromClass "/Game/Blueprints/Maps/BP_FireBall_1.BP_FireBall_1_C" (Math|Transform|MakeTransform (Math|Vector|MakeVector (.x (.location _returnvalue_15)) (- (.y (.location _returnvalue_15)) (Variables|Default|GetYVar3)) (+ (.z (.location _returnvalue_15)) (Variables|Default|GetZVar3))) (.rotation _returnvalue_15) (.scale _returnvalue_15)) "Undefined" "MultiplyWithRoot" 0 0)
  (Utilities|FlowControl|Delay 0.2)
  (Game|SpawnActorfromClass "/Game/Blueprints/Maps/BP_FireBall_1.BP_FireBall_1_C" (Math|Transform|MakeTransform (Math|Vector|MakeVector (.x (.location _returnvalue_16)) (- (.y (.location _returnvalue_16)) (Variables|Default|GetYVar2)) (+ (.z (.location _returnvalue_16)) (Variables|Default|GetZVar2))) (.rotation _returnvalue_16) (.scale _returnvalue_16)) "Undefined" "MultiplyWithRoot" 0 0)
  (Utilities|FlowControl|Delay 0.2)
  (Game|SpawnActorfromClass "/Game/Blueprints/Maps/BP_FireBall_1.BP_FireBall_1_C" (Math|Transform|MakeTransform (Math|Vector|MakeVector (.x (.location _returnvalue_17)) (- (.y (.location _returnvalue_17)) (Variables|Default|GetYVar1)) (+ (.z (.location _returnvalue_17)) (Variables|Default|GetZVar1))) (.rotation _returnvalue_17) (.scale _returnvalue_17)) "Undefined" "MultiplyWithRoot" 0 0)
  (Utilities|FlowControl|Delay 0.2)
  (Game|SpawnActorfromClass "/Game/Blueprints/Maps/BP_FireBall_1.BP_FireBall_1_C" (Math|Transform|MakeTransform (Math|Vector|MakeVector (.x (.location _returnvalue_6)) (- (.y (.location _returnvalue_6)) (Variables|Default|GetYVar2)) (+ (.z (.location _returnvalue_6)) (Variables|Default|GetZVar2))) (.rotation _returnvalue_6) (.scale _returnvalue_6)) "Undefined" "MultiplyWithRoot" 0 0)
  (Utilities|FlowControl|Delay 0.2)
  (Game|SpawnActorfromClass "/Game/Blueprints/Maps/BP_FireBall_1.BP_FireBall_1_C" (Math|Transform|MakeTransform (Math|Vector|MakeVector (.x (.location _returnvalue_5)) (- (.y (.location _returnvalue_5)) (Variables|Default|GetYVar3)) (+ (.z (.location _returnvalue_5)) (Variables|Default|GetZVar3))) (.rotation _returnvalue_5) (.scale _returnvalue_5)) "Undefined" "MultiplyWithRoot" 0 0)
  (Utilities|FlowControl|Delay 0.2)
  (Game|SpawnActorfromClass "/Game/Blueprints/Maps/BP_FireBall_1.BP_FireBall_1_C" (Math|Transform|MakeTransform (Math|Vector|MakeVector (.x (.location _returnvalue_4)) (+ (Variables|Default|GetYVar4) (.y (.location _returnvalue_4))) (+ (.z (.location _returnvalue_4)) (Variables|Default|GetZVar4))) (.rotation _returnvalue_4) (.scale _returnvalue_4)) "Undefined" "MultiplyWithRoot" 0 0)
  (Utilities|FlowControl|Delay 0.2)
  (Game|SpawnActorfromClass "/Game/Blueprints/Maps/BP_FireBall_1.BP_FireBall_1_C" (Math|Transform|MakeTransform (Math|Vector|MakeVector (.x (.location _returnvalue_13)) (+ (Variables|Default|GetYVar5) (.y (.location _returnvalue_13))) (+ (.z (.location _returnvalue_13)) (Variables|Default|GetZVar5))) (.rotation _returnvalue_13) (.scale _returnvalue_13)) "Undefined" "MultiplyWithRoot" 0 0)
  (Utilities|FlowControl|Delay 0.2)
  (Game|SpawnActorfromClass "/Game/Blueprints/Maps/BP_FireBall_1.BP_FireBall_1_C" (Math|Transform|MakeTransform (Math|Vector|MakeVector (.x (.location _returnvalue_3)) (+ (Variables|Default|GetYVar4) (.y (.location _returnvalue_3))) (+ (.z (.location _returnvalue_3)) (Variables|Default|GetZVar4))) (.rotation _returnvalue_3) (.scale _returnvalue_3)) "Undefined" "MultiplyWithRoot" 0 0)
  (Utilities|FlowControl|Delay 0.2)
  (Game|SpawnActorfromClass "/Game/Blueprints/Maps/BP_FireBall_1.BP_FireBall_1_C" (Math|Transform|MakeTransform (Math|Vector|MakeVector (.x (.location _returnvalue_2)) (- (.y (.location _returnvalue_2)) (Variables|Default|GetYVar3)) (+ (.z (.location _returnvalue_2)) (Variables|Default|GetZVar3))) (.rotation _returnvalue_2) (.scale _returnvalue_2)) "Undefined" "MultiplyWithRoot" 0 0)
  (Utilities|FlowControl|Delay 0.2)
  (Game|SpawnActorfromClass "/Game/Blueprints/Maps/BP_FireBall_1.BP_FireBall_1_C" (Math|Transform|MakeTransform (Math|Vector|MakeVector (.x (.location _returnvalue)) (- (.y (.location _returnvalue)) (Variables|Default|GetYVar2)) (+ (.z (.location _returnvalue)) (Variables|Default|GetZVar2))) (.rotation _returnvalue) (.scale _returnvalue)) "Undefined" "MultiplyWithRoot" 0 0)
  (Utilities|FlowControl|Delay 0.2)
  (Game|SpawnActorfromClass "/Game/Blueprints/Maps/BP_FireBall_1.BP_FireBall_1_C" (Math|Transform|MakeTransform (Math|Vector|MakeVector (.x (.location _returnvalue_8)) (- (.y (.location _returnvalue_8)) (Variables|Default|GetYVar1)) (+ (.z (.location _returnvalue_8)) (Variables|Default|GetZVar1))) (.rotation _returnvalue_8) (.scale _returnvalue_8)) "Undefined" "MultiplyWithRoot" 0 0)
  (StateTree|FinishTask true))