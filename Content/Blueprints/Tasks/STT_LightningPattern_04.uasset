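; STT_LightningPattern_04 is a State Tree task that spawns one fixed pattern of three blue lightning actors around a referenced actor.
; On entering the state it spawns BP_Lightning_Blue_3, BP_Lightning_Blue_2 and another Blue_3, copying that actor's transform with per-spawn Y and Z offset variables.
; The first two shift toward negative world Y and the third toward positive, all adding their Z offset.
; The task then immediately finishes as succeeded.
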(event EventLatentEnterState
  (params (Transition :type State%20Tree%20Transition%20Result%20Structure%20%28by%20ref%29))
  (bind _123 (Variables|Context|Get123))
  (bind _123_2 (Variables|Context|Get123))
  (bind _123_3 (Variables|Context|Get123))
  (bind _returnvalue (Transformation|GetActorTransform _123_3))
  (bind _returnvalue_2 (Transformation|GetActorTransform _123))
  (bind _returnvalue_3 (Transformation|GetActorTransform _123_2))
  (Game|SpawnActorfromClass "/Game/Blueprints/Maps/BP_Lightning_Blue_3.BP_Lightning_Blue_3_C" (Math|Transform|MakeTransform (Math|Vector|MakeVector (.x (.location _returnvalue)) (- (.y (.location _returnvalue)) (Variables|Default|GetYvar1)) (+ (.z (.location _returnvalue)) (Variables|Default|GetZvar1))) (.rotation _returnvalue) (.scale _returnvalue)) "Undefined" "MultiplyWithRoot" 0 0)
  (Game|SpawnActorfromClass "/Game/Blueprints/Maps/BP_Lightning_Blue_2.BP_Lightning_Blue_2_C" (Math|Transform|MakeTransform (Math|Vector|MakeVector (.x (.location _returnvalue_2)) (- (.y (.location _returnvalue_2)) (Variables|Default|GetYvar2)) (+ (.z (.location _returnvalue_2)) (Variables|Default|GetZvar2))) (.rotation _returnvalue_2) (.scale _returnvalue_2)) "Undefined" "MultiplyWithRoot" 0 0)
  (Game|SpawnActorfromClass "/Game/Blueprints/Maps/BP_Lightning_Blue_3.BP_Lightning_Blue_3_C" (Math|Transform|MakeTransform (Math|Vector|MakeVector (.x (.location _returnvalue_3)) (+ (Variables|Default|GetYvar3) (.y (.location _returnvalue_3))) (+ (.z (.location _returnvalue_3)) (Variables|Default|GetZvar3))) (.rotation _returnvalue_3) (.scale _returnvalue_3)) "Undefined" "MultiplyWithRoot" 0 0)
  (StateTree|FinishTask true))