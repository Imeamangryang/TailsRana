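; StateTree task that spawns a lightning pattern of BP_Lightning_Blue actors, noted in the graph as four zigzag electric wires.
; On latent state entry, a loop places LightningCount actors along world Y from a reference actor named "123", using spacing and offset variables plus a fixed Z offset.
; Each spawn copies that actor's rotation and scale.
; FinishTask(true) sits inside the loop body, so it is called after every spawn.
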(event EventLatentEnterState
  (params (Transition :type State%20Tree%20Transition%20Result%20Structure%20%28by%20ref%29))
  (bind _123 (Variables|context|Get123))
  (bind _returnvalue (Transformation|GetActorTransform _123))
  ;[0.15 0.15 0.15 0.5] 지그재그 전깃줄 4개 소환
  (for _index (range 0 (- (Variables|Default|GetLightning%20Count) 1))
    (Game|SpawnActorfromClass "/Game/Blueprints/Maps/BP_Lightning_Blue.BP_Lightning_Blue_C" (Math|Transform|MakeTransform (Math|Vector|MakeVector (.x (.location _returnvalue)) (- (+ (* _index (Variables|Default|GetLightning%20Pos)) (.y (.location _returnvalue))) (Variables|Default|GetYVal)) (+ (.z (.location _returnvalue)) (Variables|Default|GetZVal))) (.rotation _returnvalue) (.scale _returnvalue)) "Undefined" "MultiplyWithRoot" 0 0)
    (StateTree|FinishTask true)))