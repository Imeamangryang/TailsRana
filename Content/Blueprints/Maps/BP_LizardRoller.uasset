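; BP_LizardRoller is a moving hazard: a lizard rolling an egg that hits the player.
; On BeginPlay, the LizardForward timeline offsets the actor from its start position along the negative forward vector, while Tick pitches Scene1 by Speed to roll the egg.
; Player-tagged actors trigger a Niagara hit effect and the character's Collision function on Lizard_Collision begin overlap, but on Capsule123 end overlap.
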(event OnComponentEndOverlap(Capsule123)
  (params (OverlappedComponent :type Primitive%20Component%20Object%20Reference) (OtherActor :type Actor%20Object%20Reference) (OtherComp :type Primitive%20Component%20Object%20Reference) (OtherBodyIndex :type Integer))
  ;[0.15 0.15 0.15 0.5] 충돌시 태그가 Player 일때, Collsion 함수 실행
  (if (Actor|ActorHasTag OtherActor "Player")
    (bind _asbp_third_person_character (Utilities|Casting|CastToBP_ThirdPersonCharacter OtherActor))
    (Niagara|SpawnSystematLocation "/Game/Assets/SSR/NS_BasicHit_2.NS_BasicHit_2" (Transformation|GetActorLocation _asbp_third_person_character) "0, 0, 0" "2.000000,2.000000,2.000000")
    (Default|Collision _asbp_third_person_character)))

(event OnComponentBeginOverlap(Lizard_Collision)
  (params (OverlappedComponent :type Primitive%20Component%20Object%20Reference) (OtherActor :type Actor%20Object%20Reference) (OtherComp :type Primitive%20Component%20Object%20Reference) (OtherBodyIndex :type Integer) (bFromSweep :type Boolean) (SweepResult :type Hit%20Result%20Structure%20%28by%20ref%29))
  ;[0.15 0.15 0.15 0.5] 충돌시 태그가 Player 일때, Collsion 함수 실행
  (if (Actor|ActorHasTag OtherActor "Player")
    (bind _asbp_third_person_character (Utilities|Casting|CastToBP_ThirdPersonCharacter OtherActor))
    (Niagara|SpawnSystematLocation "/Game/Assets/SSR/NS_BasicHit_2.NS_BasicHit_2" (.Location (Collision|BreakHitResult SweepResult)) "0, 0, 0" "2.000000,2.000000,2.000000")
    (Default|Collision _asbp_third_person_character)))

(event EventBeginPlay
  ;[0.15 0.15 0.15 0.5] 앞으로 이동하는 모션
  (Utilities|FlowControl|Sequence
    (:then_0
      (Variables|Default|SetInitLocation (Transformation|GetActorLocation))
      (bind _newtrack_1 (Timeline|LizardForward Play)
        (:Update
          (Transformation|SetActorLocation (+ (Variables|Default|GetInitLocation) (* (Math|Vector|GetForwardVector (Variables|Default|GetScene)) (* _newtrack_1 -5e+02))) false false))))))

(event Collision|EventActorBeginOverlap
  (params (OtherActor :type Actor%20Object%20Reference)))

(event EventTick
  (params (DeltaSeconds :type Float%20%28single-precision%29))
  ;[0.15 0.15 0.15 0.5] 알 굴러가는 모습
  (Transformation|AddWorldRotation (Variables|Default|GetScene1) (Math|Rotator|MakeRotator 0.0 (Variables|Default|GetSpeed) 0.0) false false))

(fn ConstructionScript)