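; Fireball map hazard that moves along a timeline-driven path and hits the player on contact.
; BeginPlay starts two timelines, and SinFunction's update places the actor from its start location using ForwardTrack for backward travel and SinFunction for vertical offset along the Sphere's axes.
; Overlapping a Player-tagged character spawns a Niagara hit effect and calls that character's Collision function.
; The lifespan call is unconnected.
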(event OnComponentBeginOverlap(sphere_collision)
  (params (OverlappedComponent :type Primitive%20Component%20Object%20Reference) (OtherActor :type Actor%20Object%20Reference) (OtherComp :type Primitive%20Component%20Object%20Reference) (OtherBodyIndex :type Integer) (bFromSweep :type Boolean) (SweepResult :type Hit%20Result%20Structure%20%28by%20ref%29))
  ;[0.15 0.15 0.15 0.5] 충돌시 태그가 Player 일때, Collsion 함수 실행
  (if (Actor|ActorHasTag OtherActor "Player")
    (bind _asbp_third_person_character (Utilities|Casting|CastToBP_ThirdPersonCharacter OtherActor))
    (Niagara|SpawnSystematLocation "/Game/Assets/SSR/NS_BasicHit_2.NS_BasicHit_2" (Transformation|GetActorLocation _asbp_third_person_character) "0, 0, 0" "2.000000,2.000000,2.000000")
    (Default|Collision _asbp_third_person_character)))

(event EventBeginPlay
  ;[0.15 0.15 0.15 0.5] 불공 모션 구현
  (Utilities|FlowControl|Sequence
    (:then_0
      (Variables|Default|SetInitLocation (Transformation|GetActorLocation))
      (bind _newtrack_0 (Timeline|ForwardTrack Play)))
    (:then_1
      (Variables|Default|SetInitLocation (Transformation|GetActorLocation))
      (bind _newtrack_0_2 (Timeline|sin%20function Play)
        (:Update
          (Transformation|SetActorLocation (+ (Variables|Default|GetInitLocation) (+ (* (Math|Vector|GetForwardVector (Variables|Default|GetSphere)) (* _newtrack_0 -5e+02)) (* (Math|Vector|GetUpVector (Variables|Default|GetSphere)) (* _newtrack_0_2 4e+02)))) false false))))))

(event EventTick
  (params (DeltaSeconds :type Float%20%28single-precision%29)))

(fn ConstructionScript)