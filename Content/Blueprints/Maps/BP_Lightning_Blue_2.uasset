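; BP_Lightning_Blue_2 is a moving electric-line hazard that reacts when it touches the player.
; On BeginPlay, the ForWardTrack timeline offsets it backward along the mesh's forward vector from its start.
; A sideways ZigZagTrack term is added, but that timeline's Play is unwired, as are the lifespan and hum sound.
; Capsule overlap with a "Player"-tagged character plays a jump montage and calls that character's Collision.
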(event OnBeginCursorOver(StaticMesh)
  (params (TouchedComponent :type Primitive%20Component%20Object%20Reference)))

(event OnComponentBeginOverlap(Capsule)
  (params (OverlappedComponent :type Primitive%20Component%20Object%20Reference) (OtherActor :type Actor%20Object%20Reference) (OtherComp :type Primitive%20Component%20Object%20Reference) (OtherBodyIndex :type Integer) (bFromSweep :type Boolean) (SweepResult :type Hit%20Result%20Structure%20%28by%20ref%29))
  (if (Actor|ActorHasTag OtherActor "Player")
    (bind _asbp_third_person_character (Utilities|Casting|CastToBP_ThirdPersonCharacter OtherActor))
    (Animation|Montage|PlayMontage (Variables|/Script/Engine.Character|GetMesh (Game|GetPlayerCharacter 0)) "/Game/Blueprints/Anime/VRM_M_Joyful_Jump_Montage.VRM_M_Joyful_Jump_Montage"
      (:then
        (Default|Collision _asbp_third_person_character)))))

(event EventBeginPlay
  ;[0.15 0.15 0.15 0.5] 전기줄이 대각선방향으로 지그재그로 움직임
  (Utilities|FlowControl|Sequence
    (:then_0
      (Variables|Default|SetInitLocation (Transformation|GetActorLocation))
      (bind _newtrack_0 (Timeline|ForWardTrack Play)
        (:Update
          (Transformation|SetActorLocation (+ (Variables|Default|GetInitLocation) (+ (* (Math|Vector|GetForwardVector (Variables|Default|GetStaticMesh)) (* _newtrack_0 -5e+02)) (* (Math|Vector|GetRightVector (Variables|Default|GetStaticMesh)) (* (stale _newtrack_0) 2e+02)))) false false))))))

(event Collision|EventActorBeginOverlap
  (params (OtherActor :type Actor%20Object%20Reference)))

(event EventTick
  (params (DeltaSeconds :type Float%20%28single-precision%29)))

(fn ConstructionScript)