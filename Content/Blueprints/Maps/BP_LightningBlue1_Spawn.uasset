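; Spawner actor that periodically creates rows of BP_Lightning_Blue actors, noted in the graph as zigzag electric wires.
; Tick accumulates delta time until it reaches CreateTime, then resets the timer and rerolls CreateTime randomly between Min and Max.
; Each cycle spawns LightningCount actors using the spawner's transform, offset along world Y in LightningPos steps.
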(event EventBeginPlay)

(event Collision|EventActorBeginOverlap
  (params (OtherActor :type Actor%20Object%20Reference)))

(event EventTick
  (params (DeltaSeconds :type Float%20%28single-precision%29))
  (bind _returnvalue (Transformation|GetActorTransform))
  (bind _output_get (Variables|Default|SetCurrTime (+ DeltaSeconds (Variables|Default|GetCurrTime))))
  (if (>= _output_get (Variables|Default|GetCreateTime))
    (Variables|Default|SetCurrTime 0.0)
    (Variables|Default|SetCreateTime (Math|Random|RandomFloatinRange (Variables|Default|GetMin) (Variables|Default|GetMax)))
    ;[0.15 0.15 0.15 0.5] 지그재그 전깃줄 4개 소환
    (for _index (range 0 (- (Variables|Default|GetLightningCount) 1))
      (Game|SpawnActorfromClass "/Game/Blueprints/Maps/BP_Lightning_Blue.BP_Lightning_Blue_C" (Math|Transform|MakeTransform (Math|Vector|MakeVector (.x (.location _returnvalue)) (+ (* _index (Variables|Default|GetLightningPos)) (.y (.location _returnvalue))) (.z (.location _returnvalue))) (.rotation _returnvalue) (.scale _returnvalue)) "Undefined" "MultiplyWithRoot" 0 0))))

(fn ConstructionScript)