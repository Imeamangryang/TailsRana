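; BP_LightningBlue4_Spawn is a map actor that repeatedly spawns blue lightning actors (BP_Lightnig_Blue_4) at its own location.
; Tick accumulates delta time until it reaches CreateTime, then spawns the lightning and resets the timer.
; After each spawn, CreateTime is re-rolled randomly between the Min and Max variables, so strikes recur at irregular intervals.
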(event EventBeginPlay)

(event Collision|EventActorBeginOverlap
  (params (OtherActor :type Actor%20Object%20Reference)))

(event EventTick
  (params (DeltaSeconds :type Float%20%28single-precision%29))
  (bind _output_get (Variables|Default|SetCurrTime (+ DeltaSeconds (Variables|Default|GetCurrTime))))
  (if (>= _output_get (Variables|Default|GetCreateTime))
    (Game|SpawnActorfromClass "/Game/Blueprints/Maps/BP_Lightnig_Blue_4.BP_Lightnig_Blue_4_C" (Math|Conversions|ToTransform(Vector) (Transformation|GetActorLocation)) "Undefined" "MultiplyWithRoot" 0 0)
    (Variables|Default|SetCurrTime 0.0)
    (Variables|Default|SetCreateTime (Math|Random|RandomFloatinRange (Variables|Default|Getmin) (Variables|Default|Getmax)))))

(fn ConstructionScript)